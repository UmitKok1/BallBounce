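; Game mode for a Breakout-style paddle-and-ball game that runs the match state machine from ready through countdown, play, pause and end screens.
; It counts Brick actors on BeginPlay, and when DecrementBrickCount empties that count the level completes.
; Tick drives the three-second countdown, while SetGameState handles delayed transitions using the Paddle's lives and the GameInstance's level number.
; Completed levels open the next by name; game over or final completion shows a play-again widget.
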(event `self.ReceiveBeginPlay`
  (set `self.StateOfTheGame` "NewEnumerator0")
  (bind _outactors (`GameplayStatics.GetAllActorsOfClass` "/Game/Blueprints/Character/Brick.Brick_C"))
  (for _ _outactors
    (`/Engine/EditorBlueprintResources/StandardMacros.IncrementInt` (`self.BrickCount`))))

(event `self.ReceiveTick`
  (params (DeltaSeconds :type "Float (single-precision)"))
  ;[1 1 1] Event Tick
  (if (`|EnumEquality` (`self.StateOfTheGame`) "NewEnumerator1")
    (bind _output_get (set `self.Countdown` (- (`self.Countdown`) DeltaSeconds)))
    (if (>= _output_get 2.0)
      (set `self.Count` 3)
      (elif (>= _output_get 1.0)
        (set `self.Count` 2)
        (elif (>= _output_get 0.0)
          (set `self.Count` 1)
          (else
            (`self.SetGameState` "NewEnumerator5")))))))

(event `SetGameState`
  (params (NewParam :type "/Game/Blueprints/StateOfGame Enum" :default "NewEnumerator0"))
  (bind _returnvalue (`GameplayStatics.GetPlayerController` 0))
  (switch `/Game/Blueprints/StateOfGame` NewParam
    (:`NewEnumerator0`
      ;[1 1 1] Ready?
      (set `self.StateOfTheGame` NewParam))
    (:`NewEnumerator1`
      ;[1 1 1] Countdown
      (set `self.Countdown` 3.0)
      (set `self.StateOfTheGame` "NewEnumerator1"))
    (:`NewEnumerator2`
      ;[1 1 1] Oops!
      (set `self.StateOfTheGame` "NewEnumerator2")
      (`KismetSystemLibrary.Delay` 1.5)
      (bind _aspaddle (cast `/Game/Blueprints/Character/Paddle` (`GameplayStatics.GetPlayerPawn` 0)))
      (if (<= (`/Game/Blueprints/Character/Paddle.BallLives` _aspaddle) 0)
        (`self.SetGameState` "NewEnumerator3")
        (else
          (`self.SetGameState` "NewEnumerator0"))))
    (:`NewEnumerator3`
      ;[1 1 1] Game Over
      (set `self.StateOfTheGame` "NewEnumerator3")
      (`KismetSystemLibrary.Delay` 1.5)
      (`self.AskPlayAgain`)
      (set `PlayerController.bShowMouseCursor` true _returnvalue)
      (`WidgetBlueprintLibrary.SetInputMode_UIOnlyEx` _returnvalue null))
    (:`NewEnumerator4`
      ;[1 1 1] Level Completed
      (set `self.StateOfTheGame` "NewEnumerator4")
      (`KismetSystemLibrary.Delay` 1.5)
      (bind _asball_game_instance (cast `/Game/Blueprints/BallGameInstance` (`GameplayStatics.GetGameInstance`)))
      (bind _currentlevel (`/Game/Blueprints/BallGameInstance.CurrentLevel` _asball_game_instance))
      (if (== _currentlevel (`/Game/Blueprints/BallGameInstance.MaxLevel` _asball_game_instance))
        (`self.SetGameState` "NewEnumerator7")
        (`KismetSystemLibrary.PrintString` "Hello")
        (else
          (bind _result (`/Engine/EditorBlueprintResources/StandardMacros.IncrementInt` _currentlevel)
            (:`  `
              (`GameplayStatics.OpenLevel` (`KismetStringLibrary.Conv_StringToName` (`KismetStringLibrary.Concat_StrStr` "Level_" (`KismetStringLibrary.Conv_IntToString` _result)))))))))
    (:`NewEnumerator5`
      ;[1 1 1] Playing
      (`self.StartPlaying`)
      (set `self.StateOfTheGame` "NewEnumerator5"))
    (:`NewEnumerator6`
      ;[1 1 1] Paused
      (set `self.StateOfTheGame` "NewEnumerator6")
      (`GameplayStatics.SetGamePaused` true))
    (:`NewEnumerator7`
      ;[1 1 1] Game Completed!
      (set `self.StateOfTheGame` "NewEnumerator7")
      (`KismetSystemLibrary.Delay` 1.5)
      (`self.AskPlayAgain`))))

(fn `AskPlayAgain`
  (bind _returnvalue (`|CreateWidget` "/Game/Blueprints/HUD/PlayAgainWidget.PlayAgainWidget_C"))
  (bind _output_get (set `self.AskWidget` _returnvalue))
  (`UserWidget.AddToViewport` _output_get 0)
  (set `PlayerController.bShowMouseCursor` true (`GameplayStatics.GetPlayerController` 0)))

(fn `DecrementBrickCount`
  (bind _result (`/Engine/EditorBlueprintResources/StandardMacros.DecrementInt` (`self.BrickCount`))
    (:`  `
      (if (<= _result 0)
        (`self.SetGameState` "NewEnumerator4")))))

(fn `UserConstructionScript`)