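; Player paddle for a ball game, moved sideways along world Y by the MouseLeftRight input axis.
; Input applies only in one specific BallGameMode state, as a swept world offset scaled from the axis value.
; Helper checks compare position to LeftLimit and RightLimit, so a paddle past either limit can only move back inward.
; It also holds the BallLives count, with DecrementLives lowering it without going below zero.
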(event `InputAxis|MouseLeftRight`
  (params (AxisValue :type "Float (single-precision)"))
  (bind _asball_game_mode (cast `/Game/Blueprints/BallGameMode` (`GameplayStatics.GetGameMode`)))
  (if (`|EnumEquality` (`/Game/Blueprints/BallGameMode.StateOfTheGame` _asball_game_mode) "NewEnumerator5")
    (set `self.AxisValue` AxisValue)
    (if (`self.IsLessThan`)
      (if (`self.AxisGreaterThanZero`)
        (`self.K2_AddActorWorldOffset` (`KismetMathLibrary.MakeVector` 0.0 (* (`self.AxisValue`) 40.0)) true :!label _label))
      (elif (`self.IsGreaterThan`)
        (if (`self.AxisLessThanZero`)
          (goto _label))
        (else
          (goto _label))))))

(fn `AxisGreaterThanZero`
  (returns (AxisGreaterThanZero :type Boolean))
  (return (> (`self.AxisValue`) 0.0)))

(fn `AxisLessThanZero`
  (returns (AxisLessThanZero :type Boolean))
  (return (< (`self.AxisValue`) 0.0)))

(fn `DecrementLives`
  (if (not (< (- (`self.BallLives`) 1) 0))
    (`/Engine/EditorBlueprintResources/StandardMacros.DecrementInt` (`self.BallLives`))))

(fn `IsGreaterThan`
  (returns (GreaterThanLimit :type Boolean))
  (return (> (.y (`self.K2_GetActorLocation`)) (`self.RightLimit`))))

(fn `IsLessThan`
  (returns (LessThanLimit :type Boolean))
  (return (< (.y (`self.K2_GetActorLocation`)) (`self.LeftLimit`))))

(fn `UserConstructionScript`)