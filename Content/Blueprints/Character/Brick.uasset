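; Brick is a destructible block for a ball-and-brick game that takes several ball hits to break.
; On BeginPlay it creates a BrickNumber widget with a reference to itself and shows it in its NumberComponent.
; Each HitbyBall event lowers the hit points and plays a retro impact sound.
; The final hit decrements the BallGameMode brick count, adds a point to PlayerScore in BallGameInstance and destroys the actor.
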(event `self.ReceiveBeginPlay`
  (bind _returnvalue (`|CreateWidget` "/Game/Blueprints/HUD/BrickNumber.BrickNumber_C"))
  (set `/Game/Blueprints/HUD/BrickNumber.RefToBrick` self _returnvalue)
  (`WidgetComponent.SetWidget` (`self.NumberComponent`) _returnvalue))

(event `/Game/Blueprints/BallHitInterface.HitByBall`
  (`self.DecrementHitpoints`)
  (`GameplayStatics.PlaySound2D` "/Game/Retro_8Bit_Sounds/Impacts/Cues/retro_impact_hit_11_Cue.retro_impact_hit_11_Cue" 1.0 1.0 0.0 null null))

(fn `DecrementHitpoints`
  (if (<= (- (`self.HitPoints`) 1) 0)
    (bind _asball_game_mode (cast `/Game/Blueprints/BallGameMode` (`GameplayStatics.GetGameMode`)))
    (`/Game/Blueprints/BallGameMode.DecrementBrickCount` _asball_game_mode)
    (bind _asball_game_instance (cast `/Game/Blueprints/BallGameInstance` (`GameplayStatics.GetGameInstance`)))
    (`/Engine/EditorBlueprintResources/StandardMacros.IncrementInt` (`/Game/Blueprints/BallGameInstance.PlayerScore` _asball_game_instance)
      (:`  `
        (`self.K2_DestroyActor`)))
    (else
      (`/Engine/EditorBlueprintResources/StandardMacros.DecrementInt` (`self.HitPoints`)))))

(fn `UserConstructionScript`)